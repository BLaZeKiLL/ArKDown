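; Terrain tile for an infinite terrain mode that scatters props when play begins and manages the player's passage through it.
; Entering TileVolume turns the barrier green and passable to pawns; leaving turns it red and blocking, then asks the game mode to spawn a tile.
; DestroyVolume removes the tile when the player overlaps it.
; GetAttachPointTransform exposes the AttachPoint's world transform.
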(event `self.ReceiveBeginPlay`
  (`self.GenerateActors`))

(event `self.TileVolume.OnComponentBeginOverlap`
  (params (OverlappedComponent :type "PrimitiveComponent Object Reference") (OtherActor :type "Actor Object Reference") (OtherComp :type "PrimitiveComponent Object Reference") (OtherBodyIndex :type Integer) (bFromSweep :type Boolean) (SweepResult :type "HitResult Structure (by ref)"))
  (if (== OtherActor (`GameplayStatics.GetPlayerCharacter` 0))
    (`self.Unlock`)))

(event `self.TileVolume.OnComponentEndOverlap`
  (params (OverlappedComponent :type "PrimitiveComponent Object Reference") (OtherActor :type "Actor Object Reference") (OtherComp :type "PrimitiveComponent Object Reference") (OtherBodyIndex :type Integer))
  (if (== OtherActor (`GameplayStatics.GetPlayerCharacter` 0))
    (`self.Lock`)
    (bind _asbp_infinite_terrain_game_mode (cast `/Game/Blueprints/BP_InfiniteTerrainGameMode` (`GameplayStatics.GetGameMode`)))
    (`/Game/Blueprints/BP_InfiniteTerrainGameMode.SpawnTile` _asbp_infinite_terrain_game_mode)))

(event `self.DestroyVolume.OnComponentBeginOverlap`
  (params (OverlappedComponent :type "PrimitiveComponent Object Reference") (OtherActor :type "Actor Object Reference") (OtherComp :type "PrimitiveComponent Object Reference") (OtherBodyIndex :type Integer) (bFromSweep :type Boolean) (SweepResult :type "HitResult Structure (by ref)"))
  (if (== OtherActor (`GameplayStatics.GetPlayerCharacter` 0))
    (`self.K2_DestroyActor`)))

(fn `GenerateActors`
  (`self.PlaceActors` "/Game/Terrain/Props/BP_Container.BP_Container_C" 1 3)
  (`self.PlaceActors` "/Game/Terrain/Props/BP_Box01.BP_Box01_C" 1 3)
  (`self.PlaceActors` "/Game/Terrain/Props/BP_Box02.BP_Box02_C" 2 4)
  (`self.PlaceActors` "/Game/Terrain/Props/BP_Canister.BP_Canister_C" 3 7)
  (`self.PlaceActors` "/Game/Terrain/Props/BP_SackWall.BP_SackWall_C" 1 4)
  (`self.PlaceActors` "/Game/Terrain/Props/BP_Rock01.BP_Rock01_C" 1 4)
  (`self.PlaceActors` "/Game/Terrain/Props/BP_Rock02.BP_Rock02_C" 1 4)
  (`self.PlaceActors` "/Game/Terrain/Props/BP_Rock03.BP_Rock03_C" 1 4))

(fn `GetAttachPointTransform`
  (returns (AttachPointTransform :type "Transform Structure"))
  (return (`SceneComponent.K2_GetComponentToWorld` (`self.AttachPoint`))))

(fn `Lock`
  (bind _barrier (`self.Barrier`))
  (`PrimitiveComponent.SetCollisionResponseToChannel` _barrier "ECC_Pawn" "ECR_Block")
  (`PrimitiveComponent.SetMaterial` _barrier 0 "/Game/Terrain/MI_Red_Barrier.MI_Red_Barrier"))

(fn `Unlock`
  (bind _barrier (`self.Barrier`))
  (`PrimitiveComponent.SetCollisionResponseToChannel` _barrier "ECC_Pawn" "ECR_Ignore")
  (`PrimitiveComponent.SetMaterial` _barrier 0 "/Game/Terrain/MI_Green_Barrier.MI_Green_Barrier"))

(fn `UserConstructionScript`)