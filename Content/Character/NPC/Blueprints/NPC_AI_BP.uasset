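; NPC AI controller that feeds perceived non-enemy actors to the enemy behavior tree.
; On BeginPlay it initializes the enemy blackboard and runs the Enemy_AI behavior tree.
; AI perception updates write any sensed actor lacking the "Enemy" tag to the EnemyKey blackboard entry as the target.
; A lost stimulus from such an actor clears that key, whichever actor it currently holds.
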(event `self.ReceiveBeginPlay`
  ;[1 1 1] Begin Play
  (bind _blackboardcomponent (`self.UseBlackboard` "/Game/Character/NPC/AI/Enemy_AI_BlackBoard.Enemy_AI_BlackBoard"))
  (`self.RunBehaviorTree` "/Game/Character/NPC/AI/Enemy_AI.Enemy_AI")
  (set `self.BlackboardComponent` _blackboardcomponent))

(event `self.AIPerception.OnTargetPerceptionUpdated`
  (params (Actor :type "Actor Object Reference") (Stimulus :type "AIStimulus Structure"))
  (bind _enemy_key (`self.Enemy Key`))
  (bind _blackboardcomponent (`self.BlackboardComponent`))
  ;[1 1 1] Perception
  (if (`self.ActorHasTag` Actor "Enemy")
    _
    (elif (`.bSuccessfullySensed` (break `AIStimulus` Stimulus))
      (`BlackboardComponent.SetValueAsObject` _blackboardcomponent _enemy_key Actor)
      (else
        (`BlackboardComponent.ClearValue` _blackboardcomponent _enemy_key)))))

(fn `UserConstructionScript`)