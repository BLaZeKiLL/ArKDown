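; AIC_Enemy is the AI controller for enemy characters, running their behavior tree and tracking targets they perceive.
; On BeginPlay it sets up the BB_Enemy blackboard, starts BT_Enemy and stores the blackboard component.
; Perception updates write any sensed actor without the "Enemy" tag to the blackboard's EnemyKey, and clear that key when sensing of such an actor fails.
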(event `self.ReceiveBeginPlay`
  ;[1 1 1] Begin Play
  (bind _blackboardcomponent (`self.UseBlackboard` "/Game/Character/Enemy/AI/BB_Enemy.BB_Enemy"))
  (`self.RunBehaviorTree` "/Game/Character/Enemy/AI/BT_Enemy.BT_Enemy")
  (set `self.BlackboardComponent` _blackboardcomponent))

(event `self.AIPerception.OnTargetPerceptionUpdated`
  (params (Actor :type "Actor Object Reference") (Stimulus :type "AIStimulus Structure"))
  (bind _enemy_key (`self.Enemy Key`))
  (bind _blackboardcomponent (`self.BlackboardComponent`))
  ;[1 1 1] Perception
  (if (`self.ActorHasTag` Actor "Enemy")
    _
    (elif (`.bSuccessfullySensed` (break `AIStimulus` Stimulus))
      (`BlackboardComponent.SetValueAsObject` _blackboardcomponent _enemy_key Actor)
      (else
        (`BlackboardComponent.ClearValue` _blackboardcomponent _enemy_key)))))

(fn `UserConstructionScript`)